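; Shotgun bullet actor Blueprint that currently adds no active behavior of its own in its graphs.
; Its events are empty or disabled, and the construction script only calls the parent.
; An unconnected chain would, after a short delay, spawn a random handful of copies at jittered positions around itself.
; It clears SpawnBullets on each copy, apparently to prevent recursive spawning, but never runs.
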(event EventBeginPlay
  (|CallParentFunction) ; This node is disabled and will not be called.\nDrag off pins to build functionality.
)

(event Collision|EventActorBeginOverlap
  (params (OtherActor :type Actor%20Object%20Reference)))

(event EventTick
  (params (DeltaSeconds :type Float%20%28single-precision%29)))

(event EventRadialDamage
  (params (BaseDamage :type Float%20%28single-precision%29) (Origin :type Vector%20%28by%20ref%29 :default "0, 0, 0") (DamageRadius :type Float%20%28single-precision%29)))

(fn ConstructionScript
  (|CallParentFunction))