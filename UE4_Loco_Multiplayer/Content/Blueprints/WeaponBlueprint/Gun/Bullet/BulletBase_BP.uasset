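; Base bullet actor that ignores the player's movement collision and expires after five seconds.
; Capsule overlap damages non-player actors, adds the dealt damage to the player's Energy and destroys the bullet.
; Mesh hits play impact effects and destroy it, with optional radial impulse and pawn damage via sphere trace.
; In radial mode, Damage ticks down over flight and divides each pawn's distance, so farther pawns take more damage.
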(event OnComponentBeginOverlap(Capsule)
  (params (OverlappedComponent :type Primitive%20Component%20Object%20Reference) (OtherActor :type Actor%20Object%20Reference) (OtherComp :type Primitive%20Component%20Object%20Reference) (OtherBodyIndex :type Integer) (bFromSweep :type Boolean) (SweepResult :type Hit%20Result%20Structure%20%28by%20ref%29))
  (CallFunction|DamageActor OtherActor))

(event OnComponentHit(StaticMesh)
  (params (HitComponent :type Primitive%20Component%20Object%20Reference) (OtherActor :type Actor%20Object%20Reference) (OtherComp :type Primitive%20Component%20Object%20Reference) (NormalImpulse :type Vector :default "0, 0, 0") (Hit :type Hit%20Result%20Structure%20%28by%20ref%29))
  (bind _returnvalue (Transformation|GetActorLocation))
  (Effects|SpawnEmitteratLocation (Variables|Default|Getimpact%20Particle) _returnvalue)
  (Audio|PlaySoundatLocation (Variables|Default|GetHit%20Sound) _returnvalue)
  (Utilities|FlowControl|Sequence
    (:then_0
      (if (Variables|Default|GetDo%20Raidal%20Damage)
        (CallFunction|RadialDamage (Variables|Default|GetDamage) (Transformation|GetActorLocation) 5e+02)))
    (:then_1
      (Actor|DestroyActor))))

(event Custom|Radial%20Damage
  (params (BaseDamage :type Float%20%28single-precision%29) (Origin :type Vector%20%28by%20ref%29) (DamageRadius :type Float%20%28single-precision%29))
  (bind _outhits (Collision|MultiSphereTraceForObjects Origin Origin DamageRadius (Utilities|Array|MakeArray "ObjectTypeQuery3") false 0 "None"))
  (for _array_element _outhits
    (Class|RadialForceComponent|FireImpulse (Variables|Default|GetRadialForce))
    (Game|Damage|ApplyDamage (.HitActor (Collision|BreakHitResult _array_element)) (/ (Math|Vector|VectorLength (- (Transformation|GetActorLocation (.HitActor (Collision|BreakHitResult _array_element))) (Transformation|GetActorLocation))) (Variables|Default|GetDamage)) 0 0)))

(event Custom|Damage%20Actor
  (params (DamagedActor :type Actor%20Object%20Reference))
  (Utilities|Casting|CastToPlayer_CharacterBP DamagedActor
    (:CastFailed
      (bind _returnvalue (Game|Damage|ApplyDamage DamagedActor (Variables|Default|GetDamage) 0 0))
      (bind _asplayer_character_bp (Utilities|Casting|CastToPlayer_CharacterBP (Variables|Default|GetPlayer%20Ref)))
      (Variables|/Game/Blueprints/PlayerBlueprint/Player_CharacterBP.Player_CharacterBP_C|SetEnergy _asplayer_character_bp (+ (Variables|/Game/Blueprints/PlayerBlueprint/Player_CharacterBP.Player_CharacterBP_C|GetEnergy _asplayer_character_bp) _returnvalue))
      (Actor|DestroyActor))))

(event EventBeginPlay
  (Actor|SetLifeSpan 5.0)
  (Collision|IgnoreActorwhenMoving (Variables|Default|GetStaticMesh) (Game|GetPlayerCharacter 0) true)
  (if (Variables|Default|GetDo%20Raidal%20Damage)
    (Utilities|FlowControl|RetriggerableDelay 0.1 :!label _label)
    (Math|Float|DecrementFloat (Variables|Default|GetDamage)
      (:%20%20
        (goto _label)))))

(fn ConstructionScript)