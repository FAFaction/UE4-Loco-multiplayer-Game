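; Base gun Blueprint that fires for the player in single, burst, auto or shotgun mode, chosen by FiringType.
; Fire caches the player's mesh and camera, then each mode calls SpawnBullet, which spends player Energy and adds random recoil, scaled up while moving.
; Bullets spawn at the muzzle, aimed by a trace toward the camera's forward point, with gun and player animations.
; Reload refills Ammo from MaxAmmo, though live firing never consumes Ammo.
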(event Custom|Reload
  ;[1 1 1] Realoading
  (Variables|Default|SetReloading true)
  (Default|ADSMode (Variables|Default|GetPlayer%20Ref) false)
  (if (< (Variables|GunSettings|GetAmmo) (Variables|GunSettings|GetClip%20Size))
    (Utilities|FlowControl|Sequence
      (:then_0
        (Components|Animation|PlayAnimation (Variables|Default|GetGun%20Mesh) (Variables|Anims|GetGun%20Reaload%20Anim) false)
        (Animation|Montage|PlayMontage (Variables|Default|GetPlayer%20Mesh) (Variables|Anims|GetPlayAnim%20Reload)
          (:OnCompleted
            (Variables|Default|SetReloading false)
            (if (> (Variables|GunSettings|GetMax%20Ammo) (Variables|GunSettings|GetClip%20Size))
              (Variables|GunSettings|SetMax%20Ammo (- (Variables|GunSettings|GetMax%20Ammo) (- (Variables|GunSettings|GetClip%20Size) (Variables|GunSettings|GetAmmo))))
              (Variables|GunSettings|SetAmmo (Variables|GunSettings|GetClip%20Size))
              (else
                (Variables|GunSettings|SetAmmo (Variables|GunSettings|GetMax%20Ammo))
                (Variables|GunSettings|SetMax%20Ammo 0)))))))))

(event Custom|Fire%20Burst
  ;[1 1 1] Fire
  (Utilities|FlowControl|Sequence
    (:then_0
      _)
    (:then_1
      (Utilities|FlowControl|Delay (Variables|GunSettings|GetFire%20Rate))))
  (CallFunction|SpawnBullet))

(event Custom|Fire%20Auto
  ;[1 1 1] Fire
  (Variables|Default|SetFiring%20Auto true)
  (if (Variables|Default|GetFiring%20Auto) :!label _label
    (Utilities|FlowControl|Delay (Variables|GunSettings|GetFire%20Rate))
    (CallFunction|SpawnBullet)
    (goto _label)))

(event Custom|Stop%20Firing
  ;[1 1 1] Fire
  (Variables|Default|SetFiring%20Auto false)
  (if (Variables|Default|GetFiring%20Auto) :!label _label
    (Utilities|FlowControl|Delay (Variables|GunSettings|GetFire%20Rate))
    (CallFunction|SpawnBullet)
    (goto _label)))

(event Custom|Fire
  (params (Player%20Ref :type Character%20Object%20Reference))
  ;[1 1 1] Firing
  (bind _asplayer_character_bp (Utilities|Casting|CastToPlayer_CharacterBP Player%20Ref))
  (Variables|Default|SetPlayer%20Ref _asplayer_character_bp)
  (Variables|Default|SetPlayer%20Mesh (Variables|/Script/Engine.Character|GetMesh _asplayer_character_bp))
  (bind _camera (Default|GetPlayerCamera _asplayer_character_bp))
  (Variables|Default|SetPlayer%20Camera _camera)
  (switch Utilities|FlowControl|Switch|SwitchonE_FiringType (Variables|GunSettings|GetFiringType)
    (:NewEnumerator0
      (CallFunction|FireSingle))
    (:NewEnumerator1
      (CallFunction|FireBurst))
    (:NewEnumerator2
      (CallFunction|FireAuto))
    (:NewEnumerator3
      (CallFunction|FireShotgun))))

(event Custom|Spawn%20Bullet
  (bind _horizontal_recoil___ (Variables|GunSettings|GetHorizontal%20Recoil%20<>))
  (bind _player_ref (Variables|Default|GetPlayer%20Ref))
  (bind _player_ref_2 (Variables|Default|GetPlayer%20Ref))
  (bind _player_ref_3 (Variables|Default|GetPlayer%20Ref))
  (bind _player_ref_4 (Variables|Default|GetPlayer%20Ref))
  (bind _gun_mesh (Variables|Default|GetGun%20Mesh))
  (bind _player_camera (Variables|Default|GetPlayer%20Camera))
  (bind _returnvalue (Transformation|GetSocketLocation _gun_mesh "MuzzleFlash"))
  (bind _returnvalue_2 (Transformation|GetVelocity _player_ref_2))
  (bind _returnvalue_3 (* _horizontal_recoil___ -1.0))
  (bind _returnvalue_4 (Math|Vector|VectorLength _returnvalue_2))
  (bind _returnvalue_5 (> _returnvalue_4 0.0))
  (bind _returnvalue_6 (Math|Float|SelectFloat 2.0 1.0 _returnvalue_5))
  (if (not (Variables|Default|GetReloading))
    (if (> (Variables|/Game/Blueprints/PlayerBlueprint/Player_CharacterBP.Player_CharacterBP_C|GetEnergy _player_ref) 0.0)
      (Variables|/Game/Blueprints/PlayerBlueprint/Player_CharacterBP.Player_CharacterBP_C|SetEnergy _player_ref (- (Variables|/Game/Blueprints/PlayerBlueprint/Player_CharacterBP.Player_CharacterBP_C|GetEnergy _player_ref) (Variables|GunSettings|GetEnergy%20Cost)))
      (Utilities|FlowControl|Sequence
        (:then_0
          ;[1 1 1] Recoil
          (Pawn|Input|AddControllerPitchInput _player_ref_3 (* (Math|Random|RandomFloatinRange 0.0 (* (Variables|GunSettings|GetVertical%20Recoil%20^) _returnvalue_6)) -1.0))
          (Pawn|Input|AddControllerYawInput _player_ref_3 (Math|Random|RandomFloatinRange (* _returnvalue_3 _returnvalue_6) (* _returnvalue_3 _returnvalue_6))))
        (:then_1
          ;[1 1 1] Spawning bullets and rotating toward hit scan location
          (bind (_outhit _returnvalue_7) (Collision|LineTraceByChannel (Transformation|GetSocketLocation (Variables|Default|GetGun%20Mesh) "MuzzleFlash") (+ (Transformation|GetWorldLocation _player_camera) (* (Math|Vector|GetForwardVector _player_camera) 9e+04)) "TraceTypeQuery1" false 0 "None" true "(R=1.000000,G=0.000000,B=0.000000,A=1.000000)" "(R=0.000000,G=0.000000,B=1.000000,A=1.000000)"))
          (Game|SpawnActorfromClass (Variables|GunSettings|GetBullet%20Type) (Math|Transform|MakeTransform _returnvalue (Math|Rotator|FindLookatRotation _returnvalue (Math|Vector|SelectVector (.Location (Collision|BreakHitResult _outhit)) (.TraceEnd (Collision|BreakHitResult _outhit)) _returnvalue_7))) "AlwaysSpawn" 0 (Variables|GunSettings|GetDamage) _player_ref_4 _player_ref_4)
          (Components|Animation|PlayAnimation (Variables|Default|GetGun%20Mesh) (Variables|Anims|GetGun%20FireAnim) false)
          (Animation|Montage|PlayMontage (Variables|Default|GetPlayer%20Mesh) (Variables|Anims|GetPlayerAnim%20FireGun)))))))

(event Custom|Fire%20Shotgun
  (for _index (range 4 6)
    (CallFunction|SpawnBullet)))

(event Custom|Fire%20Single
  ;[1 1 1] Fire
  (if (not (Variables|Default|GetCan%20Fire))
    (Variables|Default|SetCan%20Fire true)
    (CallFunction|SpawnBullet)
    (Utilities|FlowControl|Delay (Variables|GunSettings|GetFire%20Rate))
    (Variables|Default|SetCan%20Fire false)))

(fn ConstructionScript)