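; Zombie enemy character that wanders the navmesh, hunts the player and fights in melee.
; Each tick while alive it checks sphere overlap, a view cone and a line trace, then either chases the player or picks random roam points, screaming on first sight.
; Close up it plays random attack montages, with hand overlaps dealing damage unless it is being hit.
; Damage updates a hit score widget, plays reactions, turns it toward the player, and at zero health triggers death montage and ragdoll.
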(event OnComponentBeginOverlap(Hand.l)
  (params (OverlappedComponent :type Primitive%20Component%20Object%20Reference) (OtherActor :type Actor%20Object%20Reference) (OtherComp :type Primitive%20Component%20Object%20Reference) (OtherBodyIndex :type Integer) (bFromSweep :type Boolean) (SweepResult :type Hit%20Result%20Structure%20%28by%20ref%29))
  (if (== OtherActor (Game|GetPlayerCharacter 0))
    (if (Variables|Default|GetAttack%20Player)
      (if (not (Variables|Default|GetBeing%20Hit))
        (Game|Damage|ApplyDamage OtherActor 1e+01 0 0)))))

(event OnComponentBeginOverlap(Hand.r)
  (params (OverlappedComponent :type Primitive%20Component%20Object%20Reference) (OtherActor :type Actor%20Object%20Reference) (OtherComp :type Primitive%20Component%20Object%20Reference) (OtherBodyIndex :type Integer) (bFromSweep :type Boolean) (SweepResult :type Hit%20Result%20Structure%20%28by%20ref%29))
  (if (== OtherActor (Game|GetPlayerCharacter 0))
    (if (Variables|Default|GetAttack%20Player)
      (if (not (Variables|Default|GetBeing%20Hit))
        (Game|Damage|ApplyDamage OtherActor 1.0 0 0)))))

(event Custom|Dead
  ;[1 1 1] WhenDead
  (Variables|Default|SetIs%20Alive false)
  (Physics|SetSimulatePhysics (Variables|Character|GetMesh) true)
  (Actor|SetLifeSpan 1e+01)
  (Collision|SetCollisionEnabled (Variables|Collision|GetCapsuleComponent) "NoCollision"))

(event Custom|Move
  (bind _returnvalue (Transformation|GetActorLocation))
  ;[1 1 1] Moving
  (if (not (Variables|Default|GetIs%20Moving))
    (Variables|Default|SetMove%20To%20Location (.RandomLocation (Class|NavigationSystem|GetRandomPointinNavigableRadius (Transformation|GetActorLocation) 5e+02)))
    (Variables|Default|SetIs%20Moving true)
    (Components|MoveComponentTo (Variables|Collision|GetCapsuleComponent) _returnvalue (Math|Rotator|MakeRotator 0.0 0.0 (.Yaw (Math|Rotator|BreakRotator (Math|Rotator|FindLookatRotation _returnvalue (Variables|Default|GetMove%20To%20Location))))) false false 0.5 true)
    (AI|AIMoveTo self (Variables|Default|GetMove%20To%20Location) 0 5.0 false
      (:OnSuccess
        (Variables|Default|SetIs%20Moving false)))))

(event Custom|Look%20for%20player
  ;[1 1 1] Look For Player
  (if (Collision|IsOverlappingActor (Variables|Default|GetSphere) (Game|GetPlayerCharacter 0) :!class /Script/Engine.PrimitiveComponent)
    (if (< (Class|KismetMathLibrary|DegAcos (Math|Vector|DotProduct (Math|Vector|Normalize (- (Transformation|GetActorLocation (Game|Player|GetPlayerPawn 0)) (Transformation|GetActorLocation))) (Transformation|GetActorForwardVector))) 4e+01)
      (bind (_outhit _returnvalue) (Collision|LineTraceByChannel (Transformation|GetActorLocation) (Transformation|GetActorLocation (Game|Player|GetPlayerPawn 0)) "TraceTypeQuery2" false 0 "ForOneFrame"))
      (if _returnvalue
        (if (== (.HitActor (Collision|BreakHitResult _outhit)) (Game|Player|GetPlayerPawn 0))
          (CallFunction|MovetoPlayer)
          (Variables|Default|Setcan%20see%20player true)
          (Utilities|FlowControl|DoOnce false :!label _label
            (:Completed
              (Animation|PlayAnimMontage "/Game/GameContent/MixamoAnims/Zombie/Montage/Zombie_Scream_Montage.Zombie_Scream_Montage" 1.0 "None")))
          (else
            (CallFunction|Move :!label _label_2)
            (Variables|Default|Setcan%20see%20player false)
            (goto _label Reset)))
        (else
          (goto _label_2)))
      (else
        (CallFunction|Move :!label _label_3)
        (Variables|Default|Setcan%20see%20player false)))
    (else
      (goto _label_3))))

(event Custom|Move%20to%20player
  ;[1 1 1] move to player & Attack player
  (if (> (Transformation|GetDistanceTo (Game|GetPlayerCharacter 0)) 1e+02)
    (AI|AIMoveTo self "0, 0, 0" (Game|Player|GetPlayerPawn 0) 5e+01 false)
    (elif (not (Variables|Default|GetAttack%20Player))
      (Variables|Default|SetAttack%20Player true)
      (Utilities|Attack
        (:Completed
          (Variables|Default|SetAttack%20Player false))))))

(event EventTick
  (params (DeltaSeconds :type Float%20%28single-precision%29))
  ;[1 1 1] Tick
  (if (Variables|Default|GetIs%20Alive)
    (CallFunction|LookforPlayer)))

(event Game|Damage|EventAnyDamage
  (params (Damage :type Float%20%28single-precision%29) (DamageType :type Damage%20Type%20Object%20Reference) (InstigatedBy :type Controller%20Object%20Reference) (DamageCauser :type Actor%20Object%20Reference))
  ;[1 1 1] Hit & Dead
  (Variables|Default|SetBeing%20Hit true)
  (if (Variables|Default|GetIs%20Alive)
    (Utilities|FlowControl|Sequence
      (:then_0
        (bind _output_get (Variables|Default|SetHealth (- (Variables|Default|GetHealth) Damage)))
        (bind _ashit_score_ui (Utilities|Casting|CastToHit_Score_UI (UserInterface|GetUserWidgetObject (Variables|Default|GetWidget))))
        (Default|Hit _ashit_score_ui (Utilities|Text|ToText(Float) Damage "HalfToEven"))
        (if (> _output_get 0.0)
          (if (> Damage 9.0)
            (Animation|PlayAnimMontage "/Game/GameContent/MixamoAnims/Zombie/Montage/Zombie_Reaction_Hit_Heavy_Montage.Zombie_Reaction_Hit_Heavy_Montage" 1.0 "None")
            (else
              (Animation|PlayAnimMontage "/Game/GameContent/MixamoAnims/Zombie/Montage/Zombie_Reaction_Hit_Light_Montage.Zombie_Reaction_Hit_Light_Montage" 1.0 "None")))
          (else
            (bind _returnvalue (Animation|PlayAnimMontage "/Game/GameContent/MixamoAnims/Zombie/Montage/Zombie_Death_Montage.Zombie_Death_Montage" 1.0 "None"))
            (Utilities|FlowControl|Delay (* _returnvalue 0.8))
            (CallFunction|Dead))))
      (:then_1
        (Transformation|SetActorRotation (CallFunction|RotationtoPlayer))
        (Utilities|FlowControl|Delay 0.3)
        (Variables|Default|SetBeing%20Hit false)))))

(event EventBeginPlay
  ;[1 1 1] Begin Play
  (CallFunction|Move))

(fn ConstructionScript
  (Class|SkinnedMeshComponent|SetMasterPoseComponent (Variables|Default|GetSkeletalMesh) (Variables|Character|GetMesh)))

(fn RotationtoPlayer
  (return (Math|Rotator|MakeRotator 0.0 0.0 (.Yaw (Math|Rotator|BreakRotator (Math|Rotator|FindLookatRotation (Transformation|GetActorLocation) (Transformation|GetActorLocation (Game|Player|GetPlayerPawn 0))))))))