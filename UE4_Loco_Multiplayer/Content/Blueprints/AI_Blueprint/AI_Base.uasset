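; Base enemy character whose behavior combines a movement type (Stalker, Guard, Coward) with an attack style (Shooter, Swinger, Puncher, Kicker).
; Tick drives both: stalkers chase, guards chase on cone-and-trace sight and wander after losing it, cowards relocate when hit.
; Shooters and swingers spawn random socketed weapons; melee uses random montages with cooldowns, and hand or foot overlaps deal damage.
; Damage updates a hit widget, plays reactions, and ragdolls on death.
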(event OnComponentBeginOverlap(HandL)
  (params (OverlappedComponent :type Primitive%20Component%20Object%20Reference) (OtherActor :type Actor%20Object%20Reference) (OtherComp :type Primitive%20Component%20Object%20Reference) (OtherBodyIndex :type Integer) (bFromSweep :type Boolean) (SweepResult :type Hit%20Result%20Structure%20%28by%20ref%29))
  ;[1 1 1] HIt Player With Punching And Kicking
  (bind _asplayer_character_bp (Utilities|Casting|CastToPlayer_CharacterBP OtherActor))
  (if (Utilities|Enum|Equal(Enum) (Variables|Attributes|GetEnemyAttribute's) "NewEnumerator2")
    (if (Variables|Default|GetHit%20Enemy%20?)
      (Game|Damage|ApplyDamage _asplayer_character_bp (Math|Random|RandomFloatinRange 2.0 5.0) 0 0))))

(event OnComponentBeginOverlap(HandR)
  (params (OverlappedComponent :type Primitive%20Component%20Object%20Reference) (OtherActor :type Actor%20Object%20Reference) (OtherComp :type Primitive%20Component%20Object%20Reference) (OtherBodyIndex :type Integer) (bFromSweep :type Boolean) (SweepResult :type Hit%20Result%20Structure%20%28by%20ref%29))
  ;[1 1 1] HIt Player With Punching And Kicking
  (bind _asplayer_character_bp (Utilities|Casting|CastToPlayer_CharacterBP OtherActor))
  (if (Utilities|Enum|Equal(Enum) (Variables|Attributes|GetEnemyAttribute's) "NewEnumerator2")
    (if (Variables|Default|GetHit%20Enemy%20?)
      (Game|Damage|ApplyDamage _asplayer_character_bp (Math|Random|RandomFloatinRange 2.0 5.0) 0 0))))

(event OnComponentBeginOverlap(FootL)
  (params (OverlappedComponent :type Primitive%20Component%20Object%20Reference) (OtherActor :type Actor%20Object%20Reference) (OtherComp :type Primitive%20Component%20Object%20Reference) (OtherBodyIndex :type Integer) (bFromSweep :type Boolean) (SweepResult :type Hit%20Result%20Structure%20%28by%20ref%29))
  ;[1 1 1] HIt Player With Punching And Kicking
  (bind _asplayer_character_bp (Utilities|Casting|CastToPlayer_CharacterBP OtherActor))
  (if (Utilities|Enum|Equal(Enum) (Variables|Attributes|GetEnemyAttribute's) "NewEnumerator3")
    (if (Variables|Default|GetHit%20Enemy%20?)
      (Game|Damage|ApplyDamage _asplayer_character_bp (Math|Random|RandomFloatinRange 5.0 8.0) 0 0))))

(event OnComponentBeginOverlap(FootR)
  (params (OverlappedComponent :type Primitive%20Component%20Object%20Reference) (OtherActor :type Actor%20Object%20Reference) (OtherComp :type Primitive%20Component%20Object%20Reference) (OtherBodyIndex :type Integer) (bFromSweep :type Boolean) (SweepResult :type Hit%20Result%20Structure%20%28by%20ref%29))
  ;[1 1 1] HIt Player With Punching And Kicking
  (bind _asplayer_character_bp (Utilities|Casting|CastToPlayer_CharacterBP OtherActor))
  (if (Utilities|Enum|Equal(Enum) (Variables|Attributes|GetEnemyAttribute's) "NewEnumerator3")
    (if (Variables|Default|GetHit%20Enemy%20?)
      (Game|Damage|ApplyDamage _asplayer_character_bp (Math|Random|RandomFloatinRange 5.0 8.0) 0 0))))

(event Custom|Get%20Away%20From%20Player
  ;[1 1 1] Move Away From Player  ONLY for Cowards
  (Variables|/Script/Engine.CharacterMovementComponent|SetMaxWalkSpeed (Variables|Character|GetCharacterMovement) 5.4e+02)
  (AI|AIMoveTo self (.RandomLocation (Class|NavigationSystem|GetRandomPointinNavigableRadius (Transformation|GetActorLocation (Game|GetPlayerCharacter 0)) 1e+03)) 0 5.0 false
    (:OnSuccess
      _)
    (:OnFail
      _))
  (Variables|/Script/Engine.CharacterMovementComponent|SetMaxWalkSpeed (Variables|Character|GetCharacterMovement) 2.7e+02)
  (Variables|Default|SetCoward%20Being%20Hit false))

(event Custom|Kick
  ;[1 1 1] Kicking
  (if (< (CallFunction|DistancetoPlayer) 1.5e+02)
    (Transformation|SetActorRotation (CallFunction|RotaiontoPlayer))
    (if (not (Variables|Default|GetAttacking))
      (Variables|Default|SetAttacking true)
      (bind _returnvalue (Animation|PlayAnimMontage (Utilities|Array|Get(acopy) (Variables|AttackComboss|GetKick%20Comboos) (Math|Random|RandomIntegerinRange 0 1)) 1.0 "None"))
      (Utilities|FlowControl|Delay _returnvalue)
      (Utilities|FlowControl|Delay (Math|Random|RandomFloatinRange 2.0 1e+01))
      (Variables|Default|SetAttacking false))))

(event Custom|Go%20to%20player
  ;[1 1 1] Go to player
  (AI|AIMoveTo self "0, 0, 0" (Game|GetPlayerCharacter 0) (Utilities|Select :Index (Variables|Attributes|GetEnemyAttribute's) :NewEnumerator0 5e+02 :NewEnumerator1 2e+02 :NewEnumerator2 1e+02 :NewEnumerator3 1e+02) false))

(event Custom|Can%20Hit%20Enemy
  (params (Hit%20? :type Boolean))
  ;[0 0 1] Hit Enable
  (Variables|Default|SetHit%20Enemy%20? Hit%20?))

(event Custom|Look%20for%20player
  ;[1 1 1] Change Movement If player has been seen
  (if (Utilities|Enum|Equal(Enum) (Variables|Attributes|GetEnemyType) "NewEnumerator1")
    (if (< (Class|KismetMathLibrary|DegAcos (Math|Vector|DotProduct (Math|Vector|Normalize (- (Transformation|GetActorLocation (Game|Player|GetPlayerPawn 0)) (Transformation|GetActorLocation))) (Transformation|GetActorForwardVector))) 4e+01)
      (bind _outhit (Collision|LineTraceByChannel (Transformation|GetActorLocation) (Transformation|GetActorLocation (Game|Player|GetPlayerPawn 0)) "TraceTypeQuery2" false 0 "None"))
      (if (== (.HitActor (Collision|BreakHitResult _outhit)) (Game|GetPlayerCharacter 0))
        (Variables|Attributes|SetCan%20See%20Player true)
        (CallFunction|GotoPlayer)
        (goto _label Reset)
        (else
          _)))
    (Variables|Attributes|SetCan%20See%20Player false)
    (Utilities|FlowControl|DoOnce false :!label _label
      (:Completed
        (Utilities|FlowControl|Delay 5.0)
        (CallFunction|Petroling)))))

(event Custom|petroling
  ;[1 1 1] Petrolling the Area
  (if (not (Variables|Attributes|GetCan%20See%20Player))
    (AI|AIMoveTo self (.RandomLocation (AI|Navigation|GetRandomReachablePointinRadius (Transformation|GetActorLocation) 1e+03)) 0 5.0 false
      (:OnSuccess
        (Utilities|FlowControl|Delay 2.0)
        (CallFunction|Petroling)))))

(event Custom|Punch
  ;[1 1 1] Punching
  (if (< (CallFunction|DistancetoPlayer) 1.5e+02)
    (Transformation|SetActorRotation (CallFunction|RotaiontoPlayer))
    (if (not (Variables|Default|GetAttacking))
      (Variables|Default|SetAttacking true)
      (bind _returnvalue (Animation|PlayAnimMontage (Utilities|Array|Get(acopy) (Variables|AttackComboss|GetPunchComboos) (Math|Random|RandomIntegerinRange 0 2)) 1.0 "None"))
      (Utilities|FlowControl|Delay _returnvalue)
      (Utilities|FlowControl|Delay (Math|Random|RandomFloatinRange 2.0 5.0))
      (Variables|Default|SetAttacking false))))

(event Custom|Coward%20Update
  ;[1 1 1] Updating Coward Movement
  (if (Variables|Default|GetCoward%20Being%20Hit)
    (Utilities|FlowControl|DoOnce false :!label _label
      (:Completed
        (CallFunction|GetAwayfromPlayer)))
    (else
      (goto _label Reset))))

(event Custom|Swing%20Weapon
  (bind _melee_weapon_ref (Variables|Default|GetMelee%20Weapon%20Ref))
  (bind _comboo (Variables|/Game/Blueprints/AI_Blueprint/AI_Weapons/Meele/AI_MeeleWeaponBase.AI_MeeleWeaponBase_C|GetComboo _melee_weapon_ref))
  ;[1 1 1] Swinging Melee Weapons
  (if (< (CallFunction|DistancetoPlayer) 3e+02)
    (Transformation|SetActorRotation (CallFunction|RotaiontoPlayer))
    (if (not (Variables|Default|GetAttacking))
      (Variables|Default|SetAttacking true)
      (bind _returnvalue (Animation|PlayAnimMontage (Utilities|Array|Get(acopy) _comboo (Math|Random|RandomIntegerinRange 0 (- (Utilities|Array|Length _comboo) 1))) 1.0 "None"))
      (Utilities|FlowControl|Delay _returnvalue)
      (Utilities|FlowControl|Delay (Math|Random|RandomFloatinRange 6.0 15.0))
      (Variables|Default|SetAttacking false))))

(event Custom|Shoot
  (bind _gun_ref (Variables|Default|GetGun%20Ref))
  (bind _enemytype (Variables|Attributes|GetEnemyType))
  ;[1 1 1] Shooting
  (if (Utilities|Enum|Equal(Enum) _enemytype "NewEnumerator1")
    (if (Variables|Attributes|GetCan%20See%20Player)
      (Transformation|SetActorRotation (CallFunction|RotaiontoPlayer) :!label _label)
      (Utilities|IsValid _gun_ref
        (:Is%20Valid
          (Default|CanShoot _gun_ref true self)
          (Variables|Default|SetSHooting true)))
      (else
        (Utilities|FlowControl|Delay 1.0 :!label _label_2)
        (Variables|Default|SetSHooting false)))
    (else
      (if (Utilities|Enum|Equal(Enum) _enemytype "NewEnumerator2")
        (if (Variables|Default|GetCoward%20Being%20Hit)
          (goto _label_2)
          (else
            _)))
      (Utilities|CanSeePlayerCheck
        (:true
          (goto _label))
        (:false
          (goto _label_2))))))

(event EventTick
  (params (DeltaSeconds :type Float%20%28single-precision%29))
  (if (Variables|Default|GetIs%20Alive)
    (Utilities|FlowControl|Sequence
      (:then_0
        (switch Utilities|FlowControl|Switch|SwitchonEnemy_Type (Variables|Attributes|GetEnemyType)
          (:NewEnumerator0
            (CallFunction|GotoPlayer))
          (:NewEnumerator1
            (CallFunction|LookforPlayer))
          (:NewEnumerator2
            (CallFunction|CowardUpdate))))
      (:then_1
        (switch Utilities|FlowControl|Switch|SwitchonEnemy_Attributes (Variables|Attributes|GetEnemyAttribute's)
          (:NewEnumerator0
            (CallFunction|Shoot))
          (:NewEnumerator1
            (CallFunction|SwingWeapon))
          (:NewEnumerator2
            (CallFunction|Punch))
          (:NewEnumerator3
            (CallFunction|Kick)))))))

(event EventBeginPlay
  (CallFunction|GiveWeaponifSwinger)
  (CallFunction|GiveGunifShooter))

(fn ConstructionScript)

(fn DistancetoPlayer
  (return (Transformation|GetDistanceTo (Game|Player|GetPlayerPawn 0))))

(fn RotaiontoPlayer
  (return (Math|Rotator|MakeRotator 0.0 0.0 (.Yaw (Math|Rotator|BreakRotator (Math|Rotator|FindLookatRotation (Transformation|GetActorLocation) (Transformation|GetActorLocation (Game|Player|GetPlayerPawn 0))))))))

(fn GiveWeaponifSwinger
  (if (Utilities|Enum|Equal(Enum) (Variables|Attributes|GetEnemyAttribute's) "NewEnumerator1")
    (bind _returnvalue (Game|SpawnActorfromClass (Utilities|Array|Get(acopy) (Variables|Default|GetSwinger%20Weapon%20Classes) (Math|Random|RandomIntegerinRange 0 2)) (Transformation|GetSocketTransform (Variables|Character|GetMesh) "Mele Socket" "RTS_World") "AlwaysSpawn" 0 self 0))
    (bind _output_get (Variables|Default|SetMelee%20Weapon%20Ref _returnvalue))
    (Transformation|AttachComponentToComponent _output_get (Variables|Character|GetMesh) "Mele Socket" "SnapToTarget" "SnapToTarget" "SnapToTarget" true)))

(fn GiveGunifShooter
  (bind _gunclasses (Variables|Default|GetGunClasses))
  (if (Utilities|Enum|Equal(Enum) (Variables|Attributes|GetEnemyAttribute's) "NewEnumerator0")
    (bind _returnvalue (Game|SpawnActorfromClass (Utilities|Array|Get(acopy) _gunclasses (Math|Random|RandomIntegerinRange 0 (- (Utilities|Array|Length _gunclasses) 1))) (Transformation|GetSocketTransform (Variables|Character|GetMesh) "Gun Socket" "RTS_World") "AlwaysSpawn" 0 0 0))
    (bind _output_get (Variables|Default|SetGun%20Ref _returnvalue))
    (Transformation|AttachComponentToComponent _output_get (Variables|Character|GetMesh) "Gun Socket" "SnapToTarget" "SnapToTarget" "SnapToTarget" true)))

(event Custom|Dead
  (bind _melee_weapon_ref (Variables|Default|GetMelee%20Weapon%20Ref))
  (bind _gun_ref (Variables|Default|GetGun%20Ref))
  (Utilities|FlowControl|Sequence
    (:then_0
      (Variables|Default|SetIs%20Alive false)
      (Physics|SetSimulatePhysics (Variables|Character|GetMesh) true)
      (Actor|SetLifeSpan 1e+01))
    (:then_1
      (Utilities|FlowControl|Sequence
        (:then_0
          (Utilities|IsValid _gun_ref
            (:Is%20Valid
              (Actor|DestroyActor _gun_ref))))
        (:then_1
          (Utilities|IsValid _melee_weapon_ref
            (:Is%20Valid
              (Actor|DestroyActor _melee_weapon_ref))))))))

(event Game|Damage|EventAnyDamage
  (params (Damage :type Float%20%28single-precision%29) (DamageType :type Damage%20Type%20Object%20Reference) (InstigatedBy :type Controller%20Object%20Reference) (DamageCauser :type Actor%20Object%20Reference))
  (if (Variables|Default|GetIs%20Alive)
    (bind _output_get (Variables|Default|SetHealth (- (Variables|Default|GetHealth) Damage)))
    (bind _ashit_score_ui (Utilities|Casting|CastToHit_Score_UI (UserInterface|GetUserWidgetObject (Variables|Default|GetWidget))))
    (Default|Hit _ashit_score_ui (Utilities|Text|ToText(Float) Damage "HalfToEven"))
    (if (> _output_get 0.0)
      (if (> Damage 9.0)
        (Animation|PlayAnimMontage "/Game/GameContent/Frank_Fighting_Set2/Animations/Montage/14_Frank_Hit_Heavy_Montage.14_Frank_Hit_Heavy_Montage" 1.0 "None")
        (else
          (Animation|PlayAnimMontage "/Game/GameContent/Frank_Fighting_Set2/Animations/Montage/10_Frank_Moves_Guard_Hit_Montage.10_Frank_Moves_Guard_Hit_Montage" 1.0 "None")))
      (Transformation|SetActorRotation (CallFunction|RotaiontoPlayer))
      (Variables|Default|SetCoward%20Being%20Hit true)
      (elif (> Damage 7.0)
        (if (> Damage 2e+01)
          (bind _returnvalue (Animation|PlayAnimMontage "/Game/GameContent/Frank_Fighting_Set2/Animations/Montage/15_Frank_Hit_Air_Montage.15_Frank_Hit_Air_Montage" 1.0 "None"))
          (Utilities|FlowControl|Delay (* _returnvalue 0.8))
          (else
            (bind _returnvalue_2 (Animation|PlayAnimMontage "/Game/GameContent/Frank_Fighting_Set2/Animations/Montage/17_Frank_Hit_KnockDown_Montage.17_Frank_Hit_KnockDown_Montage" 1.0 "None"))
            (Utilities|FlowControl|Delay (* _returnvalue_2 0.8))))
        (CallFunction|Dead)
        (else
          (CallFunction|Dead))))))