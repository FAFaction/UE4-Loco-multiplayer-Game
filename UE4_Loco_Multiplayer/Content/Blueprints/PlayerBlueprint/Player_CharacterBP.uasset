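; Player character with sprint, timed self speed boost, chained melee combos, aimed gunfire and HUD-linked weapon switching.
; Guns and melee weapons are child actors moved between hand and back sockets.
; Attacks face nearby AI and spend Energy, which also absorbs damage before health; externally set flags gate combo chaining and fist/foot overlap hits.
; Aiming zooms the camera; ADS blends to the gun's view or shows a sniper scope widget.
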(event Custom|Add%20energy
  (params (energy :type Float%20%28single-precision%29))
  ;[1 0.9666 0] Add Energy to player
  (Variables|Default|SetEnergy (+ energy (Variables|Default|GetEnergy))))

(event EventBeginPlay
  (bind _returnvalue (UserInterface|CreateWidget "/Game/Blueprints/PlayerBlueprint/Player_HUD.Player_HUD_C"))
  (bind _output_get (Variables|Default|SetPlayer%20HUD _returnvalue))
  (UserInterface|Viewport|AddtoPlayerScreen _output_get))

(event Game|Damage|EventAnyDamage
  (params (Damage :type Float%20%28single-precision%29) (DamageType :type Damage%20Type%20Object%20Reference) (InstigatedBy :type Controller%20Object%20Reference) (DamageCauser :type Actor%20Object%20Reference))
  ;[1 0 0] Damage
  (if (> (Variables|Default|GetEnergy) 0.0)
    (Variables|Default|SetEnergy (- (Variables|Default|GetEnergy) Damage))
    (else
      (Variables|Default|SetHeath (- (Variables|Default|GetHeath) Damage))))
  (if (> Damage 7.0)
    (Animation|PlayAnimMontage "/Game/GameContent/Frank_Fighting_Set2/Animations/Montage/14_Frank_Hit_Heavy_Montage.14_Frank_Hit_Heavy_Montage" 1.0 "None")
    (else
      (Animation|PlayAnimMontage "/Game/GameContent/Frank_Fighting_Set2/Animations/Montage/10_Frank_Moves_Guard_Hit_Montage.10_Frank_Moves_Guard_Hit_Montage" 1.0 "None")))
  (CallFunction|ResetCombo)
  (Variables|Default|SetBeing%20Hit%20? true)
  (Utilities|FlowControl|Delay 0.3)
  (Variables|Default|SetBeing%20Hit%20? false))

(event Input|AxisEvents|InputAxisMoveForward
  (params (AxisValue :type Float%20%28single-precision%29))
  ;[1 1 1] Basic Input
  (Pawn|Input|AddMovementInput (Math|Vector|GetForwardVector (Math|Rotator|MakeRotator 0.0 0.0 (.yaw (Pawn|GetControlRotation :!class /Script/Engine.Pawn)))) AxisValue false))

(event Input|AxisEvents|InputAxisMoveRight
  (params (AxisValue :type Float%20%28single-precision%29))
  ;[1 1 1] Basic Input
  (Pawn|Input|AddMovementInput (Math|Vector|GetRightVector (Math|Rotator|MakeRotator 0.0 0.0 (.yaw (Pawn|GetControlRotation :!class /Script/Engine.Pawn)))) AxisValue false))

(event Input|AxisEvents|InputAxisLookUp
  (params (AxisValue :type Float%20%28single-precision%29))
  ;[1 1 1] Basic Input
  (Pawn|Input|AddControllerPitchInput AxisValue))

(event Input|AxisEvents|InputAxisTurn
  (params (AxisValue :type Float%20%28single-precision%29))
  ;[1 1 1] Basic Input
  (Pawn|Input|AddControllerYawInput AxisValue))

(event Input|KeyboardEvents|LeftShift
  (params (Key :type Key%20Structure))
  ;[1 1 1] Sprint
  (:Pressed
    (bind _speed (Timeline|Sprint Play)
      (:Update
        (Variables|/Script/Engine.CharacterMovementComponent|SetMaxWalkSpeed (Variables|Character|GetCharacterMovement) _speed))))
  (:Released
    (Timeline|Sprint Reverse)))

(event Input|KeyboardEvents|3
  (params (Key :type Key%20Structure))
  (:Pressed
    (Variables|Default|SetCustomTimeDilation 2.0)
    (Utilities|FlowControl|Delay 1e+01)
    (Variables|Default|SetCustomTimeDilation 1.0)))

(event Custom|ADS%20Mode
  (params (AimDownSights :type Boolean))
  (bind _camera (Variables|Default|GetCamera))
  ;[1 1 1] Aim Down Sight
  (bind _output_get (Variables|Gun|SetADS AimDownSights))
  (if (Utilities|Enum|NotEqual(Enum) (Variables|Gun|GetGunType) "NewEnumerator3")
    (Game|Player|SetViewTargetwithBlend (Game|GetPlayerController 0) (select AimDownSights (Variables|/Script/Engine.ChildActorComponent|GetChildActor (Variables|Default|GetGun)) self) 0.2 "VTBlend_Linear" 0.0 false)
    (elif _output_get
      (bind _returnvalue (UserInterface|CreateWidget "/Game/Blueprints/WeaponBlueprint/Gun/SniperScopeUI.SniperScopeUI_C"))
      (UserInterface|Viewport|AddtoPlayerScreen _returnvalue 3)
      (Camera|SetFieldOfView _camera 1e+01)
      (else
        (Utilities|IsValid _returnvalue
          (:Is%20Valid
            (Widget|RemovefromParent _returnvalue)
            (Camera|SetFieldOfView _camera 9e+01)))))))

(event Custom|Can%20Hit%20Enemy
  (params (Hit%20? :type Boolean))
  ;[0 0 1] Comboo
  (Variables|Attack|SetHit%20Enemy%20? Hit%20?))

(event Custom|Reset%20Combo
  ;[0 0 1] Comboo
  (Variables|Attack|SetAttack%20chain 0)
  (Variables|Attack|SetChain%20Attack false)
  (Variables|Attack|SetAttacking false))

(event Custom|Chain%20Combo
  (params (Chain%20Attack :type Boolean))
  ;[0 0 1] Comboo
  (Variables|Attack|SetChain%20Attack Chain%20Attack))

(event Input|KeyboardEvents|T
  (params (Key :type Key%20Structure))
  ;[1 1 1] Aim Down Sight
  (:Pressed
    (if (not (Variables|Gun|GetADS))
      (if (Variables|Default|GetAiming)
        (CallFunction|ADSMode true))
      (else
        (CallFunction|ADSMode false)))))

(event Input|MouseEvents|MouseWheelDown
  (params (Key :type Key%20Structure))
  ;[1 1 1] Swap Mele Weapons
  (:Pressed
    (if (Variables|Mele|GetMele%20Switch%20Enable)
      (if (> (Variables|Mele|GetMeleWeaponSelectNum) 0)
        (Animation|PlayAnimMontage "/Game/GameContent/AnimStarterPack/Montage/Equip_Rifle_Standing_Montage.Equip_Rifle_Standing_Montage" 2.0 "None")
        (Utilities|FlowControl|Delay 0.5)
        (Weapon|EquipMelee)
        (Utilities|FlowControl|DoOnce false :!label _label
          (:Completed
            (Variables|Mele|SetMeleWeaponSelectNum (- (Variables|Mele|GetMeleWeaponSelectNum) 1))
            (ChildActorComponent|SetChildActorClass (Variables|Default|GetMele) (Utilities|Array|Get(acopy) (Variables|Mele|GetMele%20Weapons) (Variables|Mele|GetMeleWeaponSelectNum)))
            (Default|MeleWeaponSwap (Variables|/Game/Blueprints/PlayerBlueprint/Player_HUD.Player_HUD_C|GetMeleSelection_WB (Variables|Default|GetPlayer%20HUD)) self))))))
  (:Released
    (goto _label Reset)))

(event Input|KeyboardEvents|E
  (params (Key :type Key%20Structure))
  (bind _player_hud (Variables|Default|GetPlayer%20HUD))
  ;[1 1 1] Swaping Guns
  (:Pressed
    (Variables|Gun|SetGun%20Switch%20Enable true)
    (Default|GunSelectionActive _player_hud true))
  (:Released
    (Variables|Gun|SetGun%20Switch%20Enable false)
    (Default|GunSelectionActive _player_hud false)))

(event Input|MouseEvents|MiddleMouseButton
  (params (Key :type Key%20Structure))
  ;[1 1 1] Aim Down Sight
  (:Pressed
    (if (not (Variables|Gun|GetADS))
      (if (Variables|Default|GetAiming)
        (CallFunction|ADSMode true))
      (else
        (CallFunction|ADSMode false)))))

(event Input|MouseEvents|RightMouseButton
  (params (Key :type Key%20Structure))
  (bind _charactermovement (Variables|Character|GetCharacterMovement))
  ;[1 1 1] Aiming
  (:Pressed
    (Utilities|IsValid (Variables|/Script/Engine.ChildActorComponent|GetChildActor (Variables|Default|GetGun))
      (:Is%20Valid
        (Variables|Default|SetAiming true)
        (Utilities|FlowControl|Sequence
          (:then_0
            (if (not (Variables|Gun|GetGun%20mode))
              (Weapon|EquipGun)
              (Variables|Gun|SetGun%20mode true)))
          (:then_1
            (Variables|/Script/Engine.CharacterMovementComponent|SetbOrientRotationToMovement _charactermovement false)
            (Variables|/Script/Engine.CharacterMovementComponent|SetRotationRate _charactermovement "0,1000.000000, 0")
            (bind (_direction _fov _armtargetoffset) (Timeline|Zoom Play)
              (:Update
                (Camera|SetFieldOfView (Variables|Default|GetCamera) _fov)
                (Variables|/Script/Engine.SpringArmComponent|SetSocketOffset (Variables|Default|GetSpringArm) (Math|Vector|MakeVector 0.0 _armtargetoffset 0.0)))))))))
  (:Released
    (Variables|Default|SetAiming false)
    (CallFunction|ADSMode false)
    (Variables|/Script/Engine.CharacterMovementComponent|SetbOrientRotationToMovement _charactermovement true)
    (Variables|/Script/Engine.CharacterMovementComponent|SetRotationRate _charactermovement "0,360.000000, 0")
    (Timeline|Zoom Reverse)))

(event Input|KeyboardEvents|R
  (params (Key :type Key%20Structure))
  ;[1 1 1] Firing Gun
)

(event Input|MouseEvents|MouseWheelUp
  (params (Key :type Key%20Structure))
  ;[1 1 1] Swap Mele Weapons
  (:Pressed
    (if (Variables|Mele|GetMele%20Switch%20Enable)
      (if (< (Variables|Mele|GetMeleWeaponSelectNum) (- (Utilities|Array|Length (Variables|Mele|GetMele%20Weapons)) 1))
        (Animation|PlayAnimMontage "/Game/GameContent/AnimStarterPack/Montage/Equip_Rifle_Standing_Montage.Equip_Rifle_Standing_Montage" 2.0 "None")
        (Utilities|FlowControl|Delay 0.5)
        (Weapon|EquipMelee)
        (Utilities|FlowControl|DoOnce false :!label _label
          (:Completed
            (Variables|Mele|SetMeleWeaponSelectNum (+ (Variables|Mele|GetMeleWeaponSelectNum) 1))
            (ChildActorComponent|SetChildActorClass (Variables|Default|GetMele) (Utilities|Array|Get(acopy) (Variables|Mele|GetMele%20Weapons) (Variables|Mele|GetMeleWeaponSelectNum)))
            (Default|MeleWeaponSwap (Variables|/Game/Blueprints/PlayerBlueprint/Player_HUD.Player_HUD_C|GetMeleSelection_WB (Variables|Default|GetPlayer%20HUD)) self))))))
  (:Released
    (goto _label Reset)))

(event Input|MouseEvents|MouseWheelUp
  (params (Key :type Key%20Structure))
  (bind _gun (Variables|Default|GetGun))
  ;[1 1 1] Swaping Guns
  (:Pressed
    (if (Variables|Gun|GetGun%20Switch%20Enable)
      (if (< (Variables|Gun|GetGunSelectNum) (- (Utilities|Array|Length (Variables|Gun|GetGuns)) 1))
        (Animation|PlayAnimMontage "/Game/GameContent/AnimStarterPack/Montage/Equip_Rifle_Standing_Montage.Equip_Rifle_Standing_Montage" 2.0 "None")
        (Utilities|FlowControl|Delay 0.5)
        (Weapon|EquipGun)
        (Variables|Gun|SetGun%20mode true)
        (Utilities|FlowControl|DoOnce false :!label _label
          (:Completed
            (Variables|Gun|SetGunSelectNum (+ (Variables|Gun|GetGunSelectNum) 1))
            (ChildActorComponent|SetChildActorClass _gun (Utilities|Array|Get(acopy) (Variables|Gun|GetGuns) (Variables|Gun|GetGunSelectNum)))
            (bind _asgun_base_bp (Utilities|Casting|CastToGunBase_BP (Variables|/Script/Engine.ChildActorComponent|GetChildActor _gun)))
            (Variables|Gun|SetGunType (Variables|/Game/Blueprints/WeaponBlueprint/Gun/GunBase_BP.GunBase_BP_C|GetGunType _asgun_base_bp))
            (Default|GunSwap (Variables|/Game/Blueprints/PlayerBlueprint/Player_HUD.Player_HUD_C|GetGunSelection_WB (Variables|Default|GetPlayer%20HUD)) self))))))
  (:Released
    (goto _label Reset)))

(event Input|MouseEvents|MouseWheelDown
  (params (Key :type Key%20Structure))
  (bind _gun (Variables|Default|GetGun))
  ;[1 1 1] Swaping Guns
  (:Pressed
    (if (Variables|Gun|GetGun%20Switch%20Enable)
      (if (> (Variables|Gun|GetGunSelectNum) 0)
        (Animation|PlayAnimMontage "/Game/GameContent/AnimStarterPack/Montage/Equip_Rifle_Standing_Montage.Equip_Rifle_Standing_Montage" 2.0 "None")
        (Utilities|FlowControl|Delay 0.5)
        (Weapon|EquipGun)
        (Variables|Gun|SetGun%20mode true)
        (Utilities|FlowControl|DoOnce false :!label _label
          (:Completed
            (Variables|Gun|SetGunSelectNum (- (Variables|Gun|GetGunSelectNum) 1))
            (ChildActorComponent|SetChildActorClass _gun (Utilities|Array|Get(acopy) (Variables|Gun|GetGuns) (Variables|Gun|GetGunSelectNum)))
            (bind _asgun_base_bp (Utilities|Casting|CastToGunBase_BP (Variables|/Script/Engine.ChildActorComponent|GetChildActor _gun)))
            (Variables|Gun|SetGunType (Variables|/Game/Blueprints/WeaponBlueprint/Gun/GunBase_BP.GunBase_BP_C|GetGunType _asgun_base_bp))
            (Default|GunSwap (Variables|/Game/Blueprints/PlayerBlueprint/Player_HUD.Player_HUD_C|GetGunSelection_WB (Variables|Default|GetPlayer%20HUD)) self))))))
  (:Released
    (goto _label Reset)))

(event Input|MouseEvents|LeftMouseButton
  (params (Key :type Key%20Structure))
  ;[1 1 1] Mele Attack
  (:Pressed
    (if (not (Variables|Default|GetAiming))
      (Utilities|FlowControl|Sequence
        (:then_0
          (if (Variables|Gun|GetGun%20mode)
            (Weapon|EquipMelee)
            (Variables|Gun|SetGun%20mode false)))
        (:then_1
          (CallFunction|LookatEnemy)
          (bind _attackanims (CallFunction|GetAttackAnims))
          (if (not (Variables|Default|GetBeing%20Hit%20?))
            (if (Variables|Attack|GetAttacking)
              (if (Variables|Attack|GetChain%20Attack)
                (bind _attackanims_2 (CallFunction|GetAttackAnims :!label _label))
                (CallFunction|GetMeleEnergyCost)
                (Animation|PlayAnimMontage (Utilities|Array|Get(acopy) _attackanims_2 (Variables|Attack|GetAttack%20chain)) 1.0 "None")
                (Math|Integer|IncrementInt (Variables|Attack|GetAttack%20chain)
                  (:%20%20
                    (Variables|Attack|SetChain%20Attack false))))
              (else
                (Variables|Attack|SetAttacking true)
                (goto _label)))))))))

(event Input|MouseEvents|LeftMouseButton
  (params (Key :type Key%20Structure))
  ;[1 1 1] Firing Gun
  (:Pressed
    (if (Variables|Default|GetAiming)
      (bind _asgun_base_bp (Utilities|Casting|CastToGunBase_BP (Variables|/Script/Engine.ChildActorComponent|GetChildActor (Variables|Default|GetGun))))
      (Default|Fire _asgun_base_bp self)))
  (:Released
    (bind _asgun_base_bp_2 (Utilities|Casting|CastToGunBase_BP (Variables|/Script/Engine.ChildActorComponent|GetChildActor (Variables|Default|GetGun))))
    (Default|StopFiring _asgun_base_bp_2)))

(event Input|KeyboardEvents|Q
  (params (Key :type Key%20Structure))
  (bind _player_hud (Variables|Default|GetPlayer%20HUD))
  ;[1 1 1] Swap Mele Weapons
  (:Pressed
    (Variables|Mele|SetMele%20Switch%20Enable true)
    (Default|MeleSelectionActive _player_hud true))
  (:Released
    (Variables|Mele|SetMele%20Switch%20Enable false)
    (Default|MeleSelectionActive _player_hud false)))

(fn ConstructionScript)

(fn GetPlayerCamera
  (bind _camera (Variables|Default|GetCamera))
  (bind _asgun_base_bp (Utilities|Casting|CastToGunBase_BP (Variables|/Script/Engine.ChildActorComponent|GetChildActor (Variables|Default|GetGun))))
  (return (select (Utilities|Enum|Equal(Enum) (Variables|Gun|GetGunType) "NewEnumerator3") _camera (select (Variables|Gun|GetADS) (Variables|/Game/Blueprints/WeaponBlueprint/Gun/GunBase_BP.GunBase_BP_C|GetADS%20Cam _asgun_base_bp) _camera))))

(fn EquipGun
  (bind _gun (Variables|Default|GetGun))
  (bind _mele (Variables|Default|GetMele))
  (Utilities|FlowControl|Sequence
    (:then_0
      (Utilities|IsValid (Variables|/Script/Engine.ChildActorComponent|GetChildActor _gun)
        (:Is%20Valid
          (Transformation|AttachComponentToComponent _gun (Variables|Character|GetMesh) "Gun Socket" "SnapToTarget" "SnapToTarget" "SnapToTarget" true))))
    (:then_1
      (Utilities|IsValid (Variables|/Script/Engine.ChildActorComponent|GetChildActor _mele)
        (:Is%20Valid
          (Transformation|AttachComponentToComponent _mele (Variables|Character|GetMesh) "MeleBack" "SnapToTarget" "SnapToTarget" "SnapToTarget" true))))
    (:then_2
      (Variables|Gun|SetGun%20mode true)
      (Variables|Attack|SetAttack%20chain 0))))

(fn EquipMelee
  (bind _gun (Variables|Default|GetGun))
  (bind _mele (Variables|Default|GetMele))
  (Utilities|FlowControl|Sequence
    (:then_0
      (Utilities|IsValid (Variables|/Script/Engine.ChildActorComponent|GetChildActor _gun)
        (:Is%20Valid
          (Transformation|AttachComponentToComponent _gun (Variables|Character|GetMesh) "GunBack" "SnapToTarget" "SnapToTarget" "SnapToTarget" true))))
    (:then_1
      (Utilities|IsValid (Variables|/Script/Engine.ChildActorComponent|GetChildActor _mele)
        (:Is%20Valid
          (Transformation|AttachComponentToComponent _mele (Variables|Character|GetMesh) "Mele Socket" "SnapToTarget" "SnapToTarget" "SnapToTarget" true))))
    (:then_2
      (Variables|Gun|SetGun%20mode false)
      (Variables|Attack|SetAttack%20chain 0))))

(fn GetAttackAnims
  (bind _hth_attacks (Variables|Attack|GetHTH%20Attacks))
  (bind _mele (Variables|Default|GetMele))
  (bind _childactor (Variables|/Script/Engine.ChildActorComponent|GetChildActor _mele))
  (bind _asmele_weapon_base (Utilities|Casting|CastToMele_WeaponBase _childactor)
    (:then
      (return (select (Utilities|IsValid _childactor) (Variables|/Game/Blueprints/WeaponBlueprint/Mele/Mele_WeaponBase.Mele_WeaponBase_C|GetWeapon%20Anim%20set _asmele_weapon_base) _hth_attacks)))
    (:CastFailed
      (return _hth_attacks))))

(fn GetMeleEnergyCost
  (bind _mele (Variables|Default|GetMele))
  (bind _childactor (Variables|/Script/Engine.ChildActorComponent|GetChildActor _mele))
  (bind _asmele_weapon_base (Utilities|Casting|CastToMele_WeaponBase _childactor))
  (bind _output_get (Variables|Default|SetEnergy (- (Variables|Default|GetEnergy) (Math|Float|SelectFloat (Variables|/Game/Blueprints/WeaponBlueprint/Mele/Mele_WeaponBase.Mele_WeaponBase_C|GetEnergyCost _asmele_weapon_base) (Variables|Default|GetMelee%20Energy%20Cost) (Utilities|IsValid _childactor)))))
  (return _output_get))

(fn LookatEnemy
  (bind _returnvalue (Transformation|GetActorLocation))
  (bind _outhits (Collision|MultiSphereTraceForObjects _returnvalue _returnvalue 2e+02 (Utilities|Array|MakeArray "ObjectTypeQuery3") true 0 "None"))
  (bind _output_get (LocalVariables|SetHit%20Result%20Lcco _outhits))
  (for _array_element _output_get
    (bind _asai_base (Utilities|Casting|CastToAI_Base (.HitActor (Collision|BreakHitResult _array_element))))
    (if (Variables|/Game/Blueprints/AI_Blueprint/AI_Base.AI_Base_C|GetIs%20Alive _asai_base)
      (Utilities|Array|Add (LocalVariables|GetAI%20distance%20Loco) (Transformation|GetDistanceTo (.HitActor (Collision|BreakHitResult _array_element))))))
  (Utilities|IsValid (.HitActor (Collision|BreakHitResult (Utilities|Array|Get(acopy) (LocalVariables|GetHit%20Result%20Lcco) (.IndexOfMinValue (Math|Float|MinOfFloatArray (LocalVariables|GetAI%20distance%20Loco))))))
    (:Is%20Valid
      (Transformation|SetActorRotation (Math|Rotator|MakeRotator 0.0 0.0 (.Yaw (Math|Rotator|BreakRotator (Math|Rotator|FindLookatRotation (Transformation|GetActorLocation) (Transformation|GetActorLocation (.HitActor (Collision|BreakHitResult (Utilities|Array|Get(acopy) (LocalVariables|GetHit%20Result%20Lcco) (.IndexOfMinValue (Math|Float|MinOfFloatArray (LocalVariables|GetAI%20distance%20Loco)))))))))))))))

(event OnComponentBeginOverlap(Handr)
  (params (OverlappedComponent :type Primitive%20Component%20Object%20Reference) (OtherActor :type Actor%20Object%20Reference) (OtherComp :type Primitive%20Component%20Object%20Reference) (OtherBodyIndex :type Integer) (bFromSweep :type Boolean) (SweepResult :type Hit%20Result%20Structure%20%28by%20ref%29))
  (if (!= OtherActor self)
    (if (Variables|Attack|GetHit%20Enemy%20?)
      (Game|Damage|ApplyDamage OtherActor 5.0 0 0))))

(event OnComponentBeginOverlap(Footr)
  (params (OverlappedComponent :type Primitive%20Component%20Object%20Reference) (OtherActor :type Actor%20Object%20Reference) (OtherComp :type Primitive%20Component%20Object%20Reference) (OtherBodyIndex :type Integer) (bFromSweep :type Boolean) (SweepResult :type Hit%20Result%20Structure%20%28by%20ref%29))
  (if (!= OtherActor self)
    (if (Variables|Attack|GetHit%20Enemy%20?)
      (Game|Damage|ApplyDamage OtherActor 1e+01 0 0))))

(event OnComponentBeginOverlap(Handl)
  (params (OverlappedComponent :type Primitive%20Component%20Object%20Reference) (OtherActor :type Actor%20Object%20Reference) (OtherComp :type Primitive%20Component%20Object%20Reference) (OtherBodyIndex :type Integer) (bFromSweep :type Boolean) (SweepResult :type Hit%20Result%20Structure%20%28by%20ref%29))
  (if (!= OtherActor self)
    (if (Variables|Attack|GetHit%20Enemy%20?)
      (Game|Damage|ApplyDamage OtherActor 5.0 0 0))))

(event OnComponentBeginOverlap(Footl)
  (params (OverlappedComponent :type Primitive%20Component%20Object%20Reference) (OtherActor :type Actor%20Object%20Reference) (OtherComp :type Primitive%20Component%20Object%20Reference) (OtherBodyIndex :type Integer) (bFromSweep :type Boolean) (SweepResult :type Hit%20Result%20Structure%20%28by%20ref%29))
  (if (!= OtherActor self)
    (if (Variables|Attack|GetHit%20Enemy%20?)
      (Game|Damage|ApplyDamage OtherActor 1e+01 0 0))))