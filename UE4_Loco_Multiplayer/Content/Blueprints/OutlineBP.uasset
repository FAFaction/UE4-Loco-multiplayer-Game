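; Outline actor that adds a skeletal mesh component with an outline material to its parent actor, apparently as a child actor.
; The construction script finds the parent's first skeletal mesh component and snaps a new one onto it, using a dynamic instance of M_Outline_Inst in the first material slot.
; The graph sets neither a mesh asset nor a pose link on the new component.
; A static mesh check exists but never runs, and the event graph is empty.
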(event EventBeginPlay)

(event Collision|EventActorBeginOverlap
  (params (OtherActor :type Actor%20Object%20Reference)))

(event EventTick
  (params (DeltaSeconds :type Float%20%28single-precision%29)))

(fn ConstructionScript
  (bind _returnvalue (Actor|GetParentActor))
  (bind _returnvalue_2 (Actor|GetComponentsByClass _returnvalue "/Script/Engine.SkeletalMeshComponent"))
  (bind _output (Utilities|Array|Get(acopy) _returnvalue_2))
  (Utilities|IsValid _output
    (:Is%20Valid
      (bind _returnvalue_3 (AddComponent|AddSkeletalMeshComponent false))
      (Transformation|AttachComponentToComponent _returnvalue_3 _output "None" "SnapToTarget" "SnapToTarget" "SnapToTarget" true)
      (bind _returnvalue_4 (Rendering|Material|CreateDynamicMaterialInstance "/Game/StarterContent/Materials/M_Outline_Inst.M_Outline_Inst" :!class /Script/Engine.KismetMaterialLibrary))
      (Rendering|Material|SetMaterial _returnvalue_3 0 _returnvalue_4))))